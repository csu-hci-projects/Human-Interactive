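; End-of-maze platform actor that sends the player to the next maze level when their character overlaps it.
; GetNextMazeName finds the current level in the maze array held by ExperimentInstance, the game instance, and takes the following entry, with no check for the last index.
; The overlap event opens that level by name, then calls InvalidateLayoutAndVolatility on the ThirdPersonCharacter's PauseRef.
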(event Collision|EventActorBeginOverlap
  (params (OtherActor :type Actor%20Object%20Reference))
  (if (== OtherActor (Game|GetPlayerCharacter 0))
    (bind _mazename (CallFunction|GetNextMazeName))
    (Game|OpenLevel(byName) _mazename)
    (bind _asthird_person_character (Utilities|Casting|CastToThirdPersonCharacter (Game|GetPlayerCharacter 0)))
    (Class|Widget|InvalidateLayoutandVolatility (Variables|/Game/NotificationExperiment/Blueprints/ThirdPersonCharacter.ThirdPersonCharacter_C|GetPause%20Ref _asthird_person_character))))

(fn ConstructionScript)

(fn GetNextMazeName
  (bind _asexperiment_instance (Utilities|Casting|CastToExperimentInstance (Game|GetGameInstance)))
  (bind _mazes (Default|GetMazeArray _asexperiment_instance))
  (bind _returnvalue (Game|GetCurrentLevelName true))
  (if (>= (Utilities|Array|FindItem _mazes (Utilities|String|StringToName _returnvalue)) 0)
    (bind _result (Math|Integer|IncrementInt (Utilities|Array|FindItem _mazes (Utilities|String|StringToName _returnvalue)))
      (:%20%20
        (return (Utilities|Array|Get(acopy) _mazes _result))))))