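; Game instance for a notification experiment that opens the main menu level on init and holds each participant's session data.
; GetMazeArray uses the notification ID to pick one of four maze arrays.
; SaveResults writes participant ID, notification ID, notification counts and rating to a text file in the project directory, named from the two IDs.
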(event EventInit
  (Game|OpenLevel(byName) "MainMenu"))

(fn GetMazeArray
  (switch int (Variables|Default|GetNotif_ID)
    (:0
      (return (Variables|Default|GetLR_Mazes)))
    (:1
      (return (Variables|Default|GetMR_Mazes)))
    (:2
      (return (Variables|Default|GetUL_Mazes)))
    (:3
      (return (Variables|Default|GetUC_Mazes)))))

(fn SaveResults
  (bind _newparam (CallFunction|MakeFileTitle))
  (bind _content (CallFunction|MakeFileContent))
  (Class|VictoryBPFunctionLibrary|FileIOSaveStringTexttoFile (Class|BlueprintPathsLibrary|ProjectDir) _newparam _content false false))

(fn MakeFileContent
  (return (Class|VictoryBPFunctionLibrary|AppendMultiple "Participant ID: " (Utilities|String|ToString(Text) (Variables|Default|GetPrt_ID)) " 
Notification ID: " (Utilities|String|ToString(Integer) (Variables|Default|GetNotif_ID)) " 
Total Notifications: " (Utilities|String|ToString(Integer) (Variables|Default|GetTotal_Notif)) " 
Number Interacted With: " (Utilities|String|ToString(Integer) (Variables|Default|GetNum_Interacted)) " 
Participant Rating: " (Utilities|String|ToString(Integer) (Variables|Default|GetRating)))))

(fn MakeFileTitle
  (return (Class|VictoryBPFunctionLibrary|AppendMultiple (Utilities|String|ToString(Text) (Variables|Default|GetPrt_ID)) "_" (Utilities|String|ToString(Integer) (Variables|Default|GetNotif_ID)) ".txt")))